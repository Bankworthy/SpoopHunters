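; Player weapon tool Blueprint that handles ammo, firing and reloading through Primary, Secondary, Sprint and Reload input events.
; A state enum drives it: holding Secondary moves Rest to Ready, and Sprint then raises Ready to Aim.
; Firing requires ReadyToFire plus Ready or Aim, and only decrements clip ammo.
; Reloading uses a timer to refill the clip from reserve, then returns to Ready, with debug prints throughout.
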(event `self.ReceiveBeginPlay`
  (`parent.ReceiveBeginPlay`)
  (set `self.CurrentAmmo` (`self.MaxAmmo`))
  (set `self.CurrentAmmoInClip` (`self.MaxAmmoInClip`)))

(event `self.Primary`
  (if (`self.bReadyToFire`)
    (`self.FireFunction`)))

(event `self.PrimaryReleased`)

(event `self.Secondary`
  (switch `/Game/Weapons/WeaponState` (`self.State`)
    (:`NewEnumerator0`
      (set `self.State` "NewEnumerator1")
      (`KismetSystemLibrary.PrintString` (`|GetEnumeratorNameAsString` (`self.State`)) :!label _label))))

(event `self.SecondaryReleased`
  (switch `/Game/Weapons/WeaponState` (`self.State`)
    (:`NewEnumerator1`
      (set `self.State` "NewEnumerator0")
      (goto _label))))

(event `self.Reload`
  (`self.ReloadFunction`))

(event `self.Sprint`
  (switch `/Game/Weapons/WeaponState` (`self.State`)
    (:`NewEnumerator1`
      (set `self.State` "NewEnumerator2")
      (goto _label))))

(event `self.SprintReleased`
  (switch `/Game/Weapons/WeaponState` (`self.State`)
    (:`NewEnumerator2`
      (set `self.State` "NewEnumerator1")
      (goto _label))))

(fn `FireFunction`
  (if (`self.bReadyToFire`)
    (switch `/Game/Weapons/WeaponState` (`self.State`)
      (:`NewEnumerator1`
        _)
      (:`NewEnumerator2`
        _))
    (if (> (`self.CurrentAmmoInClip`) 0)
      (bind _result (`/Engine/EditorBlueprintResources/StandardMacros.DecrementInt` (`self.CurrentAmmoInClip`))
        (:`  `
          (`KismetSystemLibrary.PrintString` (`KismetStringLibrary.Conv_IntToString` _result)))))))

(fn `Reloaded`
  (bind _returnvalue (`KismetMathLibrary.Min` (`self.ClipDelta`) (`self.CurrentAmmo`)))
  (`KismetSystemLibrary.K2_ClearTimer` null "Reloaded")
  (set `self.CurrentAmmoInClip` (+ (`self.CurrentAmmoInClip`) _returnvalue))
  (set `self.CurrentAmmo` (- (`self.CurrentAmmo`) _returnvalue))
  (set `self.State` "NewEnumerator1")
  (`KismetSystemLibrary.PrintString` "DONE")
  (`KismetSystemLibrary.PrintString` (`KismetStringLibrary.Conv_IntToString` (`self.CurrentAmmoInClip`)))
  (`KismetSystemLibrary.PrintString` (`|GetEnumeratorNameAsString` (`self.State`))))

(fn `ReloadFunction`
  (if (and (!= (`self.CurrentAmmoInClip`) (`self.MaxAmmoInClip`)) (!= (`self.CurrentAmmo`) 0))
    (switch `/Game/Weapons/WeaponState` (`self.State`)
      (:`NewEnumerator0`
        _)
      (:`NewEnumerator1`
        _)
      (:`NewEnumerator2`
        _))
    (set `self.State` "NewEnumerator3")
    (set `self.ClipDelta` (- (`self.MaxAmmoInClip`) (`self.CurrentAmmoInClip`)))
    (`KismetSystemLibrary.K2_SetTimer` null "Reloaded" (`self.ReloadTime`))
    (`KismetSystemLibrary.PrintString` "Reloading")))

(fn `UserConstructionScript`
  (`parent.UserConstructionScript`))